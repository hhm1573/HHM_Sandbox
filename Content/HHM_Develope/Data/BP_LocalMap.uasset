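; BP_LocalMap is an actor that holds the tile data for a rectangular local map grid.
; On BeginPlay it calls SetMapSize with a hardcoded square size.
; SetMapSize clears any existing TileData and resizes it to width times height, storing the grid as one flat array.
; It does not fill in tile contents, and the Tick, overlap and construction graphs are empty.
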(event EventBeginPlay
  (Initialize|SetMapSize 5 5))

(event Collision|EventActorBeginOverlap
  (params (OtherActor :type Actor%20Object%20Reference)))

(event EventTick
  (params (DeltaSeconds :type Float%20%28single-precision%29)))

(fn ConstructionScript)

(fn SetMapSize
  (params (MapSize_Horizontal :type Integer) (MapSize_Vertical :type Integer))
  (bind _output_get (LocalVariables|SetArraySize (* MapSize_Horizontal MapSize_Vertical)))
  (if (== (Utilities|Array|Length (Variables|Default|GetTileData)) 0)
    _
    (else
      (Utilities|Array|Clear (Variables|Default|GetTileData))))
  (Utilities|Array|Resize (Variables|Default|GetTileData) _output_get))