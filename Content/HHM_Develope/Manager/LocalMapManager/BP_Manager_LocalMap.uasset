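; BP_Manager_LocalMap is a manager actor that creates and sizes the game's local map at play start.
; On BeginPlay it reads the horizontal and vertical map sizes from BP_GameInstance_HHM, spawns a BP_LocalMap at the world origin, keeps a reference, and passes the sizes to its SetMapSize.
; It stops early if the game instance cast fails, and has no active tick or overlap logic.
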(event EventBeginPlay
  (|CallParentFunction)
  (bind _asbp_game_instance_hhm (Utilities|Casting|CastToBP_GameInstance_HHM (Variables|Default|GetGameInstance)))
  (Variables|MapInfo|SetMapSize_Horizontal (Variables|/Game/HHM_Develope/BP_GameInstance_HHM.BP_GameInstance_HHM_C|GetMapSize_Horizontal _asbp_game_instance_hhm))
  (Variables|MapInfo|SetMapSize_Vertical (Variables|/Game/HHM_Develope/BP_GameInstance_HHM.BP_GameInstance_HHM_C|GetMapSize_Vertical _asbp_game_instance_hhm))
  (bind _returnvalue (Game|SpawnActorfromClass "/Game/HHM_Develope/Data/BP_LocalMap.BP_LocalMap_C" (Math|Transform|MakeTransform "0, 0, 0") "Undefined" 0 0))
  (bind _output_get (Variables|Default|SetLocalMap _returnvalue))
  (Default|SetMapSize _output_get (Variables|MapInfo|GetMapSize_Horizontal) (Variables|MapInfo|GetMapSize_Vertical)))

(event Collision|EventActorBeginOverlap
  (params (OtherActor :type Actor%20Object%20Reference))
  (|CallParentFunction OtherActor) ; 지금 이 노드는 비활성 상태입니다. \n핀을 끌어서 다른 노드를 연결하면 활성화됩니다.
)

(event EventTick
  (params (DeltaSeconds :type Float%20%28single-precision%29))
  (|CallParentFunction DeltaSeconds) ; 지금 이 노드는 비활성 상태입니다. \n핀을 끌어서 다른 노드를 연결하면 활성화됩니다.
)

(fn ConstructionScript
  (|CallParentFunction))