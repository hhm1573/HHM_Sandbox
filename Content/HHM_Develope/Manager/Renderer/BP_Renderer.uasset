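; BP_Renderer is an actor, apparently an unfinished renderer for tile maps using instanced static meshes.
; InitializeMeshComponent adds two instanced mesh components, a sphere and a cube, and stores them by index in ArrInstancedMesh.
; RenderMap only copies the map's TileData into RestRender without creating instances, and ClearInstance loops over the components with an empty body.
; The event graph is inactive, and nothing in the Blueprint calls these functions.
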(event EventBeginPlay
  (|CallParentFunction) ; 지금 이 노드는 비활성 상태입니다. \n핀을 끌어서 다른 노드를 연결하면 활성화됩니다.
)

(event Collision|EventActorBeginOverlap
  (params (OtherActor :type Actor%20Object%20Reference))
  (|CallParentFunction OtherActor) ; 지금 이 노드는 비활성 상태입니다. \n핀을 끌어서 다른 노드를 연결하면 활성화됩니다.
)

(event EventTick
  (params (DeltaSeconds :type Float%20%28single-precision%29))
  (|CallParentFunction DeltaSeconds) ; 지금 이 노드는 비활성 상태입니다. \n핀을 끌어서 다른 노드를 연결하면 활성화됩니다.
)

(fn ConstructionScript
  (|CallParentFunction))

(fn InitializeMeshComponent
  (Utilities|FlowControl|Sequence
    (:then_0
      (bind _returnvalue (AddComponent|AddInstancedStaticMeshComponent false))
      (Utilities|Array|SetArrayElem (Variables|RenderComp|GetArr_InstancedMesh) 0 _returnvalue)
      (Components|StaticMesh|SetStaticMesh _returnvalue "/Game/StarterContent/Props/MaterialSphere.MaterialSphere"))
    (:then_1
      (bind _returnvalue_2 (AddComponent|AddInstancedStaticMeshComponent false))
      (Utilities|Array|SetArrayElem (Variables|RenderComp|GetArr_InstancedMesh) 1 _returnvalue_2)
      (Components|StaticMesh|SetStaticMesh _returnvalue_2 "/Game/StarterContent/Shapes/Shape_Cube.Shape_Cube"))))

(fn RenderMap
  (params (LocalMap :type BP%20Local%20Map%20Object%20Reference%20%28by%20ref%29))
  (LocalVariables|SetRestRender (Variables|/Game/HHM_Develope/Data/BP_LocalMap.BP_LocalMap_C|GetTileData LocalMap)))

(fn ClearInstance
  (for _index (range 0 (- (Utilities|Array|Length (Variables|RenderComp|GetArr_InstancedMesh)) 1))
    _))