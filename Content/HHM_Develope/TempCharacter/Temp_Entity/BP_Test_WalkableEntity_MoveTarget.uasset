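; Test move-target marker for walkable entities, placed on an X/Z grid by its horizontal and vertical indices.
; BeginPlay snaps it to the center of that 100-unit cell at Y=0.
; Tick accumulates time and, after the first second, re-applies the snap every frame because the timer never resets.
; Releasing Space orders every BPTest_WalkableEntity to MoveTo the marker's indices.
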(event EventBeginPlay
  (Transformation|SetActorLocation (Math|Vector|MakeVector (Math|Conversions|ToFloat(Integer) (+ (* (Variables|Default|Getindex%20horizontal) 100) 50)) 0.0 (Math|Conversions|ToFloat(Integer) (+ (* (Variables|Default|Getindex%20vertical) 100) 50))) false false))

(event Collision|EventActorBeginOverlap
  (params (OtherActor :type Actor%20Object%20Reference)))

(event EventTick
  (params (DeltaSeconds :type Float%20%28single-precision%29))
  (bind _output_get (Variables|Default|SetDelta%20time (+ (Variables|Default|GetDelta%20time) DeltaSeconds)))
  (if (>= _output_get 1.0)
    (Transformation|SetActorLocation (Math|Vector|MakeVector (Math|Conversions|ToFloat(Integer) (+ (* (Variables|Default|Getindex%20horizontal) 100) 50)) 0.0 (Math|Conversions|ToFloat(Integer) (+ (* (Variables|Default|Getindex%20vertical) 100) 50))) false false)))

(event Input|KeyboardEvents|SpaceBar
  (params (Key :type Key%20Structure :default "None"))
  (:Released
    (bind _outactors (Actor|GetAllActorsOfClass "/Game/HHM_Develope/TempCharacter/Temp_Entity/BPTest_WalkableEntity.BPTest_WalkableEntity_C"))
    (for _array_element _outactors
      (Default|Moveto _array_element (Variables|Default|Getindex%20horizontal) (Variables|Default|Getindex%20vertical)))))

(fn ConstructionScript)